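; BP_Collectable is a collectable item actor that can show and hide a highlight on its mesh.
; Highlight spawns an unattached copy of the mesh at its world transform, with a dynamic instance of an outline material on slot 0.
; Unhighlight destroys that copy, and a flag prevents duplicate highlights.
; It holds no pickup logic, and its event graph is empty.
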(event `self.ReceiveBeginPlay`)

(fn `Highlight`
  (if (not (`self.IsHiglighted`))
    (bind _returnvalue (`AddComponent|NODE_AddStaticMeshComponent-0` :`bManualAttachment` true :`RelativeTransform` (`SceneComponent.K2_GetComponentToWorld` (`self.Mesh`))))
    (set `self.HighlightMesh` _returnvalue)
    (`StaticMeshComponent.SetStaticMesh` _returnvalue (`StaticMeshComponent.StaticMesh` (`self.Mesh`)))
    (`PrimitiveComponent.CreateDynamicMaterialInstance` _returnvalue 0 "/Game/Items/M_OutlineTest_Inst.M_OutlineTest_Inst" "None")
    (set `self.IsHiglighted` true)))

(fn `Unhighlight`
  (bind _highlightmesh (`self.HighlightMesh`))
  (set `self.IsHiglighted` false)
  (`/Engine/EditorBlueprintResources/StandardMacros.IsValid` _highlightmesh
    (:`Is Valid`
      (`ActorComponent.K2_DestroyComponent` _highlightmesh))))

(fn `UserConstructionScript`)