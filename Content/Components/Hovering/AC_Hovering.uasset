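; Actor component that makes its owner bob up and down around its starting height.
; On BeginPlay it takes the owner's primitive component, enables physics with gravity off, and stores Z limits a hovering range above and below the start.
; Each tick it flips direction on crossing a limit and applies a vertical acceleration force that way.
; Leftover debug prints are never executed.
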(event `self.ReceiveBeginPlay`
  (bind _hoveringrange (`self.HoveringRange`))
  (bind _returnvalue (`Actor.GetComponentByClass` (`self.GetOwner`) "/Script/Engine.PrimitiveComponent"))
  (bind (_returnvalue_x _returnvalue_y _returnvalue_z) (`KismetMathLibrary.BreakVector` (`SceneComponent.K2_GetComponentLocation` (`self.Owner`))))
  (`|ExecutionSequence`
    (:`then_0`
      (set `self.Owner` _returnvalue)
      (`PrimitiveComponent.SetSimulatePhysics` _returnvalue true)
      (`PrimitiveComponent.SetEnableGravity` _returnvalue false))
    (:`then_1`
      (set `self.MinDistance` (- _returnvalue_z _hoveringrange)))
    (:`then_2`
      (set `self.MaxDistance` (+ _returnvalue_z _hoveringrange)))))

(event `self.ReceiveTick`
  (params (DeltaSeconds :type "Float (single-precision)"))
  (bind _hoveringforce (`self.HoveringForce`))
  (bind (_returnvalue_x _returnvalue_y _returnvalue_z) (`KismetMathLibrary.BreakVector` (`SceneComponent.K2_GetComponentLocation` (`self.Owner`))))
  (bind (_returnvalue_x_2 _returnvalue_y_2 _returnvalue_z_2) (`KismetMathLibrary.BreakVector` (`SceneComponent.K2_GetComponentLocation` (`self.Owner`))))
  (`|ExecutionSequence`
    (:`then_0`
      (if (>= _returnvalue_z_2 (`self.MaxDistance`))
        (set `self.IsDistanceUp` false)))
    (:`then_1`
      (if (<= _returnvalue_z (`self.MinDistance`))
        (set `self.IsDistanceUp` true)))
    (:`then_2`
      (if (`self.IsDistanceUp`)
        (`PrimitiveComponent.AddForce` (`self.Owner`) (`KismetMathLibrary.MakeVector` 0.0 0.0 _hoveringforce) "None" true)
        (else
          (`PrimitiveComponent.AddForce` (`self.Owner`) (`KismetMathLibrary.MakeVector` 0.0 0.0 (* _hoveringforce -1.0)) "None" true))))))